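; BP_WindowGenerator is a construction-script tool that builds a large generic wall window of adjustable width from modular meshes.
; Length is grid-snapped by SnapScale and clamped at zero, then offsets the left and right pieces outward and stretches the middle piece, hidden at near-zero length.
; The glass pane is rescaled only while the middle shows, with a fixed scale for short spans.
; ExtendWall toggles visibility of side wall extensions, which never have collision.
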(fn `UserConstructionScript`
  (locals (SnappedLength :type "Float (double-precision)" :default 0.0))
  (bind _sm_genericwall_largewindow_middle (`self.SM_GenericWall_LargeWindow_Middle`))
  (bind _wallextensionright (`self.WallExtensionRight`))
  (bind _wallextensionleft (`self.WallExtensionLeft`))
  (bind _returnvalue (`KismetMathLibrary.GridSnap_Float` (`self.Length`) (`self.SnapScale`)))
  (if (`self.ExtendWall`)
    (`SceneComponent.SetVisibility` _wallextensionleft true false)
    (`SceneComponent.SetVisibility` (`self.WallExtensionRight`) true false)
    (`PrimitiveComponent.SetCollisionEnabled` _wallextensionleft "NoCollision")
    (`PrimitiveComponent.SetCollisionEnabled` (`self.WallExtensionRight`) "NoCollision")
    (else
      (`SceneComponent.SetVisibility` _wallextensionright false false)
      (`SceneComponent.SetVisibility` (`self.WallExtensionLeft`) false false)
      (`PrimitiveComponent.SetCollisionEnabled` _wallextensionright "NoCollision")
      (`PrimitiveComponent.SetCollisionEnabled` (`self.WallExtensionLeft`) "NoCollision")))
  (if (< _returnvalue 0.0)
    (set `local.SnappedLength` 0.0)
    (else
      (set `local.SnappedLength` _returnvalue)))
  (`SceneComponent.K2_SetRelativeLocation` (`self.SM_GenericWall_LargeWindow_Right`) (`KismetMathLibrary.MakeVector` (+ (* (`local.SnappedLength`) 100.0) 100.0)) false false)
  (`SceneComponent.K2_SetRelativeLocation` (`self.SM_GenericWall_LargeWindow_Left`) (`KismetMathLibrary.MakeVector` (+ (* (`local.SnappedLength`) -100.0) -100.0)) false false)
  (if (or (>= (`local.SnappedLength`) 0.1) (<= (`local.SnappedLength`) -0.1))
    (`SceneComponent.SetVisibility` _sm_genericwall_largewindow_middle true false)
    (`SceneComponent.SetRelativeScale3D` (`self.SM_GenericWall_LargeWindow_Middle`) (`KismetMathLibrary.MakeVector` (`local.SnappedLength`) 1.0 1.0))
    (if (>= (`local.SnappedLength`) 0.4)
      (`SceneComponent.K2_SetRelativeTransform` (`self.SM_GlassPane`) (`KismetMathLibrary.MakeTransform` (0.0 0.0 -36.0) (struct) (`KismetMathLibrary.MakeVector` (+ (`local.SnappedLength`) 1.0) 1.0 1.3)) false false)
      (else
        (`SceneComponent.K2_SetRelativeTransform` (`self.SM_GlassPane`) (`KismetMathLibrary.MakeTransform` (0.0 0.0 -36.0) (struct) (1.5 1.0 1.3)) false false)))
    (else
      (`SceneComponent.SetVisibility` _sm_genericwall_largewindow_middle false false))))