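; BP_WindowPane is a generic wall window piece whose length is adjustable.
; Its construction script snaps Length to the SnapScale grid with a minimum of one, then stretches the Window component along X by that value.
; RightEdge and LeftEdge move symmetrically outward in proportion to the snapped length, following the stretched window without being scaled by the script.
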(fn `UserConstructionScript`
  (locals (SnappedLength :type "Float (double-precision)" :default 0.0))
  (bind _snappedlength (`local.SnappedLength`))
  (bind _snappedlength_2 (`local.SnappedLength`))
  (bind _returnvalue (`KismetMathLibrary.GridSnap_Float` (`self.Length`) (`self.SnapScale`)))
  (if (< _returnvalue 1.0)
    (set `local.SnappedLength` 1.0)
    (else
      (set `local.SnappedLength` _returnvalue)))
  (`SceneComponent.SetRelativeScale3D` (`self.Window`) (`KismetMathLibrary.MakeVector` (`local.SnappedLength`) 1.0 1.0))
  (`SceneComponent.K2_SetRelativeLocation` (`self.Right Edge`) (`KismetMathLibrary.MakeVector` (+ (* _snappedlength 100.0) (* _snappedlength -15.0))) false false)
  (`SceneComponent.K2_SetRelativeLocation` (`self.Left Edge`) (`KismetMathLibrary.MakeVector` (+ (* _snappedlength_2 -100.0) (* _snappedlength_2 15.0))) false false))