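; Procedural staircase that rebuilds in the construction script from step count, spacing and width.
; Instanced Step meshes advance equally in Y and Z, while Support instances run along negative Y with increasing Z scale, one fewer than the steps.
; An optional Platform scales from grid-snapped height, width and the stored step index, read before that run recalculates width and index.
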(fn `InvertNumber`
  (params (`Positive Number` :type "Float (double-precision)"))
  (returns (`Negative Number` :type "Float (double-precision)"))
  (return (- `Positive Number` (* `Positive Number` 2.0))))

(fn `UserConstructionScript`
  (`InstancedStaticMeshComponent.ClearInstances` (`self.Support`))
  (`InstancedStaticMeshComponent.ClearInstances` (`self.Step`))
  (if (`self.UsePlatform`)
    (set `self.ActualPlatformHeight` (`KismetMathLibrary.GridSnap_Float` (/ (`self.PlatformHeight`) 10.0) 0.1))
    (`SceneComponent.SetRelativeScale3D` (`self.Platform`) (`KismetMathLibrary.MakeVector` (`self.ActualWidth`) (`KismetMathLibrary.Conv_IntToDouble` (+ (`self.Index`) 1)) (`self.ActualPlatformHeight`))))
  (set `self.ActualWidth` (`KismetMathLibrary.GridSnap_Float` (/ (`self.Staircase Width`) 10.0) 0.1))
  (if (> (`self.Steps`) 1)
    (for _index (range (`self.Steps`))
      (set `self.Index` _index)
      (bind _returnvalue (* _index (`self.DistanceBetweenStep`)))
      (`InstancedStaticMeshComponent.AddInstance` (`self.Step`) (`KismetMathLibrary.MakeTransform` (`KismetMathLibrary.MakeVector` 0.0 _returnvalue _returnvalue) (struct) (`KismetMathLibrary.MakeVector` (`self.ActualWidth`) 1.0 1.0)) false)
      (if (not (== (`self.Index`) (- (`self.Steps`) 1)))
        (`InstancedStaticMeshComponent.AddInstance` (`self.Support`) (`KismetMathLibrary.MakeTransform` (`KismetMathLibrary.MakeVector` 0.0 (`self.InvertNumber` (* (`self.DistanceBetweenStep`) (`self.Index`)))) (struct) (`KismetMathLibrary.MakeVector` (`self.ActualWidth`) 1.0 (`KismetMathLibrary.Conv_IntToDouble` (+ (`self.Index`) 1)))) false)))
    (else
      (`InstancedStaticMeshComponent.AddInstance` (`self.Step`) (`KismetMathLibrary.MakeTransform` (0.0 0.0 0.0) (struct) (`KismetMathLibrary.MakeVector` (`self.ActualWidth`) 1.0 1.0)) false))))